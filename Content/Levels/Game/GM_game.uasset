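; Game mode for the game level of a multiplayer match with Blue and Red third-person characters.
; PostLogin switches the default pawn between the two by player-count parity, records the controller and refreshes the session after a retriggerable delay; logout removes the controller.
; Tick checks the first player's O key to update the session and server-travel to the Lobby.
; Disconnected, unused chains hold server-full kicking and manual spawn-and-possess logic.
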(event `self.HandleStartingNewPlayer`
  (params (NewPlayer :type "PlayerController Object Reference")))

(event `self.ReceiveTick`
  (params (DeltaSeconds :type "Float (single-precision)"))
  (if (`PlayerController.IsInputKeyDown` (`GameplayStatics.GetPlayerController` 0) "O")
    (bind (_numconnections _numprivateconnections _bislan _bisdedicated _ballowinvites _ballowjoininprogress _bisanticheatenabled _builduniqueid _extrasettings) (`AdvancedSessionsLibrary.GetSessionSettings`)
      (:`OnSuccess`
        (`UpdateSessionCallbackProxyAdvanced.UpdateSession` _extrasettings _numconnections
          (:`OnSuccess`
            (`KismetSystemLibrary.ExecuteConsoleCommand` "serverTravel Lobby" (`GameplayStatics.GetPlayerController` (`KismetArrayLibrary.Array_Length` (`self.playerControllers`))))))))))

(event `self.K2_OnLogout`
  (params (ExitingController :type "Controller Object Reference"))
  (bind _asplayer_controller (cast `PlayerController` ExitingController))
  (`KismetArrayLibrary.Array_RemoveItem` (`self.playerControllers`) _asplayer_controller))

(event `self.K2_PostLogin`
  (params (NewPlayer :type "PlayerController Object Reference"))
  (if (== (mod (`KismetArrayLibrary.Array_Length` (`GameStateBase.PlayerArray` (`GameplayStatics.GetGameState`))) 2) 0)
    (set `self.DefaultPawnClass` "/Game/ThirdPerson/Blueprints/BP_ThirdPersonCharacterBlue.BP_ThirdPersonCharacterBlue_C")
    (else
      (set `self.DefaultPawnClass` "/Game/ThirdPerson/Blueprints/BP_ThirdPersonCharacterRed.BP_ThirdPersonCharacterRed_C")))
  (`KismetArrayLibrary.Array_AddUnique` (`self.playerControllers`) NewPlayer)
  (`KismetSystemLibrary.RetriggerableDelay` 2.0)
  (bind (_numconnections _numprivateconnections _bislan _bisdedicated _ballowinvites _ballowjoininprogress _bisanticheatenabled _builduniqueid _extrasettings) (`AdvancedSessionsLibrary.GetSessionSettings`)
    (:`OnSuccess`
      (`UpdateSessionCallbackProxyAdvanced.UpdateSession` _extrasettings _numconnections))))

(fn `UserConstructionScript`)