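; PC_Lobby is the lobby player controller, handling the player's UI and input freezing.
; Custom events create widgets for countdown, timer info, start conditions and lovers' victory, and disable or re-enable input on the controlled pawn.
; Holding Tab shows the scoreboard, while a final scoreboard event displays it briefly, then unfreezes the pawn.
; Escape toggles the menu, using mouse cursor visibility as the open state.
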(event `self.ReceiveBeginPlay`)

(event `ShowCountDown`
  (bind _returnvalue (`|CreateWidget` "/Game/Levels/Lobby/W_ShowCountDown.W_ShowCountDown_C"))
  (`UserWidget.AddToViewport` _returnvalue 0))

(event `Freeze`
  (`self.DisableInput` (`self.K2_GetPawn`) self))

(event `Unfreeze`
  (`self.EnableInput` (`self.K2_GetPawn`) self))

(event `Show_TimerInfo`
  (bind _returnvalue (`|CreateWidget` "/Game/Levels/Lobby/W_TimerInfo.W_TimerInfo_C"))
  (`UserWidget.AddToViewport` _returnvalue 0))

(event `Key|Tab`
  (params (Key :type "Key Structure"))
  (bind _scoreboard (`self.scoreBoard`))
  (:`Pressed`
    (bind _returnvalue (`|CreateWidget` "/Game/Levels/Lobby/W_ScoreBoard.W_ScoreBoard_C" null null))
    (bind _output_get (set `self.scoreBoard` _returnvalue))
    (`UserWidget.AddToViewport` _output_get 0))
  (:`Released`
    (`/Engine/EditorBlueprintResources/StandardMacros.IsValid` _scoreboard
      (:`Is Valid`
        (`Widget.RemoveFromParent` _scoreboard)))))

(event `FinalScoreBoard`
  (bind _returnvalue (`|CreateWidget` "/Game/Levels/Lobby/W_ScoreBoard.W_ScoreBoard_C" null null))
  (`UserWidget.AddToViewport` _returnvalue 0)
  (`KismetSystemLibrary.Delay` 5.0)
  (`Widget.RemoveFromParent` _returnvalue)
  (`self.Unfreeze`))

(event `LoversVictory`
  (bind _returnvalue (`|CreateWidget` "/Game/Levels/Lobby/W_ShowLoversVictory.W_ShowLoversVictory_C"))
  (`UserWidget.AddToViewport` _returnvalue 0))

(event `ConditionsToStart`
  (bind _returnvalue (`|CreateWidget` "/Game/Levels/Lobby/W_ShowConditionsToStart.W_ShowConditionsToStart_C"))
  (`UserWidget.AddToViewport` _returnvalue 0))

(event `Key|Escape`
  (params (Key :type "Key Structure"))
  (:`Pressed`
    (if (`self.bShowMouseCursor`)
      (`self.CloseMenu`)
      (else
        (`self.OpenMenu`)))))

(fn `CloseMenu`
  (bind _menu (`self.Menu`))
  (set `self.bShowMouseCursor` false)
  (`/Engine/EditorBlueprintResources/StandardMacros.IsValid` _menu
    (:`Is Valid`
      (`Widget.RemoveFromParent` _menu))))

(fn `OpenMenu`
  (set `self.bShowMouseCursor` true)
  (bind _returnvalue (`|CreateWidget` "/Game/Levels/Lobby/W_Menu.W_Menu_C"))
  (bind _output_get (set `self.Menu` _returnvalue))
  (`UserWidget.AddToViewport` _output_get 0))

(fn `UserConstructionScript`)